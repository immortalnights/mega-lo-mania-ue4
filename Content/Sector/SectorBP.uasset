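; Sector actor that shows or hides its side and corner pieces to match a layout row in the Sectors data table.
; The construction script passes MapType to RenderMap, which hides each side whose flag is set.
; Each corner shows only when both adjacent side flags are off.
; A timer event that would cycle through the table rows exists, but its setup is disconnected and never runs.
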(event Custom|CustomEvent_0
  (Variables|Default|SetMapIndex (+ (Variables|Default|GetMapIndex) 1))
  (bind _outrownames (DataTable|GetDataTableRowNames "/Game/Sector/Sectors.Sectors"))
  (CallFunction|RenderMap (Utilities|Array|Get(acopy) _outrownames (Variables|Default|GetMapIndex))))

(event EventBeginPlay)

(event EventTick
  (params (DeltaSeconds :type Float%20%28single-precision%29)))

(fn ConstructionScript
  (CallFunction|RenderMap (Variables|Default|GetMapType)))

(fn RenderMap
  (params (Map :type Name))
  (bind _returnvalue (Utilities|GetDataTableRow "/Game/Sector/Sectors.Sectors" Map)
    (:then
      ;[1 1 1] Sides
      (Rendering|SetVisibility (Variables|Default|GetTop) (not (.top _returnvalue)) true)
      (Rendering|SetVisibility (Variables|Default|GetRight) (not (.right _returnvalue)) true)
      (Rendering|SetVisibility (Variables|Default|GetBottom) (not (.bottom _returnvalue)) true)
      (Rendering|SetVisibility (Variables|Default|GetLeft) (not (.left _returnvalue)) true)
      ;[1 1 1] Corners
      (Rendering|SetVisibility (Variables|Default|GetTopRightCorner) (and (not (.top _returnvalue)) (not (.right _returnvalue))) true)
      (Rendering|SetVisibility (Variables|Default|GetBottomRightCorner) (and (not (.bottom _returnvalue)) (not (.right _returnvalue))) true)
      (Rendering|SetVisibility (Variables|Default|GetBottomLeftCorner) (and (not (.bottom _returnvalue)) (not (.left _returnvalue))) true)
      (Rendering|SetVisibility (Variables|Default|GetTopLeftCorner) (and (not (.top _returnvalue)) (not (.left _returnvalue))) true))))